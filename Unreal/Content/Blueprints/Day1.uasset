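; Day1 Blueprint that solves part one of a line-by-line digit puzzle and prints the result on BeginPlay.
; SolvePart1 reads lines from a FileReader component, joins each line's first and last digits into a number, and sums them.
; FindFirstDigit serves both ends by optionally reversing the string before scanning its characters for the first numeric one.
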(event OnComponentActivated(FileReader)
  (params (Component :type Actor%20Component%20Object%20Reference) (bReset :type Boolean)))

(event EventBeginPlay
  (bind _result (CallFunction|SolvePart1))
  (Development|PrintString _result))

(event EventTick
  (params (DeltaSeconds :type Float%20%28single-precision%29)))

(fn ConstructionScript)

(fn SolvePart1
  (LocalVariables|SetSum 0)
  (for _array_element (Class|FileReader|ReadLines (Variables|Default|GetFileReader))
    (bind _value (CallFunction|FindFirstDigit _array_element false))
    (bind _value_2 (CallFunction|FindFirstDigit _array_element true))
    (LocalVariables|SetSum (+ (LocalVariables|GetSum) (Math|Conversions|ToInteger(Byte) (Utilities|String|Append (Utilities|String|ToString(Integer) _value) (Utilities|String|ToString(Integer) _value_2))))))
  (return (Utilities|String|ToString(Integer) (LocalVariables|GetSum))))

(fn FindFirstDigit
  (params (Str :type String) (reversed :type Boolean))
  (for _array_element (Utilities|String|GetCharacterArrayfromString (Utilities|String|SelectString (Utilities|String|Reverse Str) Str reversed))
    (if (Class|KismetStringLibrary|IsNumeric _array_element)
      (LocalVariables|SetDigit (Math|Conversions|ToInteger(Byte) _array_element))
      (return (LocalVariables|GetDigit))))
  (return (LocalVariables|GetDigit)))